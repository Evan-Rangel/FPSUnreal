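; Player character for a Space Invaders game that moves sideways, fires projectiles and has health and lives.
; Fire input drives a Gate and Delay auto-fire loop with clamped rate, a lockout and an optional FlipFlop that skips alternate shots.
; Damage triggers HealthCheck for death and explosion, then RespawnPlayer resets health in place or opens the "Perdiste" level when lives run out.
; Respawn leaves capsule collision disabled, setting NoCollision both times.
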(event `InputAxis|MoveRight`
  (params (AxisValue :type "Float (single-precision)"))
  (`self.AddMovementInput` (`KismetMathLibrary.GetRightVector` (`KismetMathLibrary.MakeRotator` 0.0 0.0 (.yaw (`self.GetControlRotation`)))) AxisValue))

(event `Force-Firing_Now`
  (bind _returnvalue (`SceneComponent.GetSocketLocation` (`self.Mesh`) "SpaceInvadersPlayerSocket"))
  (if (not (`self.Lock_Firing`)) :!label _label
    (if (`self.Can_Fire`)
      (`|ExecutionSequence`
        (:`then_0`
          (goto _label_2 :!via `Open`))
        (:`then_1`
          (`/Engine/EditorBlueprintResources/StandardMacros.Gate` true :!label _label_2
            (:`Exit`
              (`|ExecutionSequence`
                (:`then_0`
                  _)
                (:`then_1`
                  (`KismetSystemLibrary.Delay` (`KismetMathLibrary.FClamp` (* (`self.Fire_Rate`) (`self.Fire_Rate_Multi`)) 0.033) :!label _label_3)
                  (set `self.Can_Fire` true)
                  (goto _label_2)))))))
      (else
        (`|ExecutionSequence`
          (:`then_0`
            (goto _label_2 :!via `Open`))
          (:`then_1`
            (goto _label_3)))))
    (if (`self.Flip_Flop_Firing`)
      (`/Engine/EditorBlueprintResources/StandardMacros.FlipFlop`
        (:`A`
          (`|SpawnActorFromClass` (`self.Proyectile`) (`KismetMathLibrary.MakeTransform` (`SceneComponent.GetSocketLocation` (`self.Mesh`) "SpaceInvadersPlayerSocket") (struct :`Yaw` 90.0)) "Undefined" "OverrideRootScale" null (`self.Damage_Multi`) 3000.0 false true null)))
      (else
        (`|SpawnActorFromClass` (`self.Proyectile`) (`KismetMathLibrary.MakeTransform` _returnvalue (struct :`Yaw` 90.0)) "Undefined" "OverrideRootScale" null (`self.Damage_Multi`) 3000.0 false true null)
        (`|SpawnActorFromClass` (`self.Proyectile`) (`KismetMathLibrary.MakeTransform` _returnvalue (struct :`Yaw` 90.0)) "Undefined" "OverrideRootScale" null (`self.Damage_Multi`) 3000.0 false true null)))
    (set `self.Can_Fire` false)))

(event `InputAction|Fire1`
  (params (Key :type "Key Structure"))
  (:`Pressed`
    (if (`self.Alive`)
      (goto _label)))
  (:`Released`
    (if (not (`self.Lock_Firing`))
      (goto _label_2 :!via `Close`))))

(event `Stop_Firing_Now`
  (params (`Look Firing Input` :type Boolean))
  (if `Look Firing Input`
    (set `self.Lock_Firing` true)
    (goto _label_2 :!via `Close`)))

(event `self.ReceiveAnyDamage`
  (params (Damage :type "Float (single-precision)") (DamageType :type "DamageType Object Reference") (InstigatedBy :type "Controller Object Reference") (DamageCauser :type "Actor Object Reference"))
  (set `self.Health` (- (`self.Health`) (* (`self.Damage_Multi`) Damage)))
  (`self.HealthCheck`)
  (if (not (`self.Alive`))
    (set `self.Vidas` (- (`self.Vidas`) 1))
    (if (>= (`self.Vidas`) 0)
      (`self.RespawnPlayer`)
      (else
        (set `self.Alive` false)
        (set `self.Fire_Rate` 0.0)))))

(fn `HealthCheck`
  (if (<= (`self.Health`) 0.0)
    (set `self.Alive` false)
    (`GameplayStatics.SpawnEmitterAtLocation` "/Game/StarterContent/Particles/P_Explosion.P_Explosion" (`self.K2_GetActorLocation`) (struct) (2.0 2.0 2.0))
    (`KismetSystemLibrary.PrintText` (`KismetTextLibrary.Conv_DoubleToText` (`self.Health`) "HalfToEven"))))

(fn `UserConstructionScript`)