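; Game mode for a Space Invaders level that spawns enemy waves, counts down a timer and tracks score.
; A recursive spawn loop reads numbered Gameplay_Data rows, passing per-enemy health, movement, firing and score settings at spawn, then waits the row's duration.
; A Delay on Tick decrements Segundos each second, opening "Perdiste" at zero.
; Puntajes adds points per call, opening "Ganaste" once the score threshold is met.
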(event `self.ReceiveTick`
  (params (DeltaSeconds :type "Float (single-precision)"))
  (`KismetSystemLibrary.Delay` 1.0)
  (if (== (`self.segundos`) 0)
    (`GameplayStatics.OpenLevel` "Perdiste")
    (else
      (set `self.segundos` (- (`self.segundos`) 1)))))

(event `self.ReceiveBeginPlay`
  (`KismetSystemLibrary.Delay` 0.2)
  (`self.Spawn_Loop`)
  (`KismetSystemLibrary.PrintString` (`KismetStringLibrary.Conv_IntToString` (`self.Score2`))))

(event `Spawn_Loop`
  (bind _returnvalue (`|GetDataTableRow` "/Game/SpaceInvaders/Personaje/Gameplay_Data.Gameplay_Data" (`KismetStringLibrary.Conv_StringToName` (`KismetStringLibrary.Conv_IntToString` (`self.Spawn_Loop_Counter`))))
    (:`then`
      (bind _output_get (set `self.Current_Row_Data` _returnvalue))
      (bind (_seq _seqduration _scene _enemycount _actor _locations _movements _health _movespeedmulti _xymulti _velocity _canshoot _firerate _projectile _scoregive) (break `/Game/SpaceInvaders/Personaje/GamePlay_Struct` _output_get))
      (set `self.Spawn_Delay` _seqduration)
      (set `self.Scene` _scene)
      (for _index (range _enemycount)
        (bind (_x _y) (`KismetMathLibrary.BreakVector2D` (`self.Safe_Get_Array_Element` _xymulti _index)))
        (bind _returnvalue_2 (`|SpawnActorFromClass` (`|GetArrayItem` (`self.Enemy_Classes`) (`self.Safe_Get_Array_Element` _actor _index)) (`KismetMathLibrary.MakeTransform` (`self.Safe_Get_Array_Element` _locations _index)) "Undefined" "OverrideRootScale" null (`self.Safe_Get_Array_Element` _health _index) (`self.Safe_Get_Array_Element` _scoregive _index) (`self.Safe_Get_Array_Element` _movements _index) (`self.Safe_Get_Array_Element` _movespeedmulti _index) _x _y (`self.Safe_Get_Array_Element` _velocity _index) (`self.Safe_Get_Array_Element` _canshoot _index) (`self.Safe_Get_Array_Element` _firerate _index) null null))
        (`KismetArrayLibrary.Array_AddUnique` (`self.Enemies_Just_Spawned`) _returnvalue_2))
      (bind _result (`/Engine/EditorBlueprintResources/StandardMacros.IncrementInt` (`self.Spawn_Loop_Counter`))
        (:`  `
          (set `self.Spawn_Loop_Counter` _result)
          (`KismetSystemLibrary.RetriggerableDelay` (`self.Spawn_Delay`))
          (`KismetArrayLibrary.Array_Clear` (`self.Enemies_Just_Spawned`))
          (`self.Spawn_Loop`))))))

(fn `Puntajes`
  (bind _score2 (`self.Score2`))
  (if (or (> _score2 1000) (== _score2 1000))
    (`GameplayStatics.OpenLevel` "Ganaste")
    (else
      (set `self.Score2` (+ (`self.Score2`) 100)))))

(fn `UserConstructionScript`)