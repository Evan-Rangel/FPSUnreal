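; BP_Dummy is a ghost enemy that chases any pawn it senses and dies to any damage with a sound and smoke puff.
; Overlapping its DamagePlayer component costs the cached BP_MasterChief one Health, without checking what overlapped.
; A DoOnce limits repeat hits, resetting two seconds after the overlap ends.
; At zero Health it runs the player death itself: sparks, hidden character, music, camera fade, then MainMenu loads.
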(event `self.ReceiveBeginPlay`
  (bind _asbp_master_chief (cast `/Game/Plataformero/Characters/MasterChief/BluePrints/BP_MasterChief` (`GameplayStatics.GetPlayerCharacter` 0)))
  (set `self.As BP Master Chief` _asbp_master_chief))

(event `self.ReceiveAnyDamage`
  (params (Damage :type "Float (single-precision)") (DamageType :type "DamageType Object Reference") (InstigatedBy :type "Controller Object Reference") (DamageCauser :type "Actor Object Reference"))
  (bind _returnvalue (`SceneComponent.K2_GetComponentLocation` (`self.StaticMesh`)))
  (`GameplayStatics.PlaySoundAtLocation` "/Game/Plataformero/Enemies/Fantasma1/Sounds/GhostDie.GhostDie" _returnvalue (struct) 1.0 1.0 0.0 null null null null)
  (`GameplayStatics.SpawnEmitterAtLocation` "/Game/StarterContent/Particles/P_Smoke.P_Smoke" _returnvalue (struct) (0.5 0.5 0.5))
  (`self.K2_DestroyActor`))

(event `self.PawnSensing.OnSeePawn`
  (params (Pawn :type "Pawn Object Reference"))
  (`AIBlueprintHelperLibrary.SimpleMoveToActor` null Pawn)
  (`KismetSystemLibrary.PrintString` "Hello"))

(event `self.DamagePlayer.OnComponentBeginOverlap`
  (params (OverlappedComponent :type "PrimitiveComponent Object Reference") (OtherActor :type "Actor Object Reference") (OtherComp :type "PrimitiveComponent Object Reference") (OtherBodyIndex :type Integer) (bFromSweep :type Boolean) (SweepResult :type "HitResult Structure (by ref)"))
  (bind _as_bp_master_chief (`self.As BP Master Chief`))
  (bind _health (`/Game/Plataformero/Characters/MasterChief/BluePrints/BP_MasterChief.Health` (`self.As BP Master Chief`)))
  (`/Engine/EditorBlueprintResources/StandardMacros.DoOnce` false :!label _label
    (:`Completed`
      (`/Engine/EditorBlueprintResources/StandardMacros.DecrementInt` _health
        (:`  `
          (if (< _health 1)
            (`GameplayStatics.SpawnEmitterAtLocation` "/Game/StarterContent/Particles/P_Sparks.P_Sparks" (`self.K2_GetActorLocation` _as_bp_master_chief) (struct) (0.3 0.3 0.3))
            (`self.SetActorHiddenInGame` _as_bp_master_chief true)
            (set `CharacterMovementComponent.MaxWalkSpeed` 0.0 (`Character.CharacterMovement` _as_bp_master_chief))
            (`GameplayStatics.PlaySound2D` "/Game/Plataformero/Enemies/Fantasma1/Sounds/DeadMusic_01.DeadMusic_01" 1.0 1.0 0.0 null null)
            (`PlayerCameraManager.StartCameraFade` :`self` (`GameplayStatics.GetPlayerCameraManager` 0) :`ToAlpha` 1.5 :`Duration` 6.2 :`bShouldFadeAudio` true)
            (`KismetSystemLibrary.Delay` 6.0)
            (`GameplayStatics.OpenLevel` "MainMenu")))))))

(event `self.DamagePlayer.OnComponentEndOverlap`
  (params (OverlappedComponent :type "PrimitiveComponent Object Reference") (OtherActor :type "Actor Object Reference") (OtherComp :type "PrimitiveComponent Object Reference") (OtherBodyIndex :type Integer))
  (`KismetSystemLibrary.Delay` 2.0)
  (goto _label :!via `Reset`))

(fn `UserConstructionScript`)