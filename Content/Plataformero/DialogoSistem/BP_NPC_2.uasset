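; BP_NPC_2 is an NPC for the platformer's dialogue system that steps through its Dialogo lines.
; Each Talk call increments TalkIndex, lazily creates a BPW_DialogoSistem widget and shows the indexed line in its TalkText.
; The widget is removed once TalkIndex exceeds the array length; the inclusive bound allows an index one past the last line.
; BeginPlay caches the player as BP_MasterChief, though Talk does not use it.
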(event `self.ReceiveBeginPlay`
  (bind _asbp_master_chief (cast `/Game/Plataformero/Characters/MasterChief/BluePrints/BP_MasterChief` (`GameplayStatics.GetPlayerCharacter` 0)))
  (set `self.As BP Master Chief` _asbp_master_chief))

(event `/Game/Plataformero/DialogoSistem/BP_DialogoSistem.Talk`
  (`/Engine/EditorBlueprintResources/StandardMacros.IncrementInt` (`self.talkIndex`)
    (:`  `
      (if (<= (`self.talkIndex`) (`KismetArrayLibrary.Array_Length` (`self.Dialogo`)))
        (`self.UI`
          (:`then`
            _)
          (:`else`
            (bind _returnvalue (`|CreateWidget` "/Game/Plataformero/Characters/MasterChief/Ui/BPW_DialogoSistem.BPW_DialogoSistem_C" (`GameplayStatics.GetPlayerController` 0)))
            (bind _output_get (set `self.UI` _returnvalue))
            (`UserWidget.AddToViewport` _output_get 0)))
        (`TextBlock.SetText` (`/Game/Plataformero/Characters/MasterChief/Ui/BPW_DialogoSistem.TalkText` (`self.UI`)) (`KismetTextLibrary.Conv_StringToText` (`|GetArrayItem` (`self.Dialogo`) (`self.talkIndex`))))
        (else
          (`Widget.RemoveFromParent` (`self.UI`)))))))

(fn `UserConstructionScript`)