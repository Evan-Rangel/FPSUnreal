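; BP_SelectLevelPlayer is the player for the platformer's level-select screen, showing the mouse cursor and sliding the camera sideways.
; Tick polls DER to play a timeline that lerps the camera's Y offset and pitch.
; Within that timeline's updates, a cleared DER lets DER2 play or reverse a second timeline, whose forward update slides the camera further along Y.
; Neither flag is set in this Blueprint.
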(event `self.ReceiveBeginPlay`
  (set `PlayerController.bShowMouseCursor` true (`GameplayStatics.GetPlayerController` 0)))

(event `self.ReceiveTick`
  (params (DeltaSeconds :type "Float (single-precision)"))
  (if (`self.DER`)
    (bind (_direction _rotar) (`Timeline|Timeline`)
      (:`Update`
        (`SceneComponent.K2_SetRelativeLocation` (`self.Camera`) (`KismetMathLibrary.MakeVector` 0.0 (`KismetMathLibrary.Lerp` 0.0 1600.0 _rotar)) false false)
        (`SceneComponent.K2_SetRelativeRotation` (`self.Camera`) (`KismetMathLibrary.MakeRotator` 0.0 (`KismetMathLibrary.Lerp` -20.0 -30.0 _rotar)) false false)
        (if (`self.DER`)
          _
          (elif (`self.DER2`)
            (bind (_direction_2 _rotar_2) (`Timeline|Timeline_0` :!label _label)
              (:`Update`
                (`SceneComponent.K2_SetRelativeLocation` (`self.Camera`) (`KismetMathLibrary.MakeVector` 0.0 (`KismetMathLibrary.Lerp` 1600.0 4000.0 _rotar_2)) false false)))
            (else
              (goto _label :!via `Reverse`))))))))

(fn `UserConstructionScript`)