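; BP_PlayerMenu is the main menu player Blueprint, which shows the mouse cursor and moves the menu camera for the options view.
; Every Tick it checks the Opciones flag and plays the RotRotate timeline forward when true, or reverses it when false.
; The timeline's Rotar track drives lerps that yaw and offset the camera's relative transform between its default and options framing.
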(event `self.ReceiveBeginPlay`
  (set `PlayerController.bShowMouseCursor` true (`GameplayStatics.GetPlayerController` 0)))

(event `self.ReceiveTick`
  (params (DeltaSeconds :type "Float (single-precision)"))
  (if (`self.Opciones`)
    (bind (_direction _rotar) (`Timeline|Rot Rotate` :!label _label)
      (:`Update`
        (`SceneComponent.K2_SetRelativeRotation` (`self.Camera`) (`KismetMathLibrary.MakeRotator` 0.0 0.0 (`KismetMathLibrary.Lerp` 0.0 45.0 _rotar)) false false)
        (`SceneComponent.K2_SetRelativeLocation` (`self.Camera`) (`KismetMathLibrary.MakeVector` (`KismetMathLibrary.Lerp` 0.0 50.0 _rotar) (`KismetMathLibrary.Lerp` 0.0 250.0 _rotar)) false false)))
    (else
      (goto _label :!via `Reverse`))))

(fn `UserConstructionScript`)