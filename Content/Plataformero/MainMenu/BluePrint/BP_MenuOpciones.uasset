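; BP_MenuOpciones is a main menu actor that slides vertically into place when the options menu is triggered.
; It caches the BP_PlayerMenu pawn on BeginPlay and polls its Opciones flag every Tick.
; The first time the flag is true, a DoOnce gate stores the start location, waits briefly, then plays a timeline that lerps only Z to a fixed height.
; The gate is never reset, so the move happens once.
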(event `self.ReceiveBeginPlay`
  (bind _asbp_player_menu (cast `/Game/Plataformero/MainMenu/BluePrint/BP_PlayerMenu` (`GameplayStatics.GetPlayerPawn` 0)))
  (set `self.As BP Player Menu` _asbp_player_menu))

(event `self.ReceiveTick`
  (params (DeltaSeconds :type "Float (single-precision)"))
  (bind (_locstart_x _locstart_y _locstart_z) (`KismetMathLibrary.BreakVector` (`self.LocStart`)))
  (if (`/Game/Plataformero/MainMenu/BluePrint/BP_PlayerMenu.Opciones` (`self.As BP Player Menu`))
    (`/Engine/EditorBlueprintResources/StandardMacros.DoOnce` false
      (:`Completed`
        (set `self.LocStart` (`self.K2_GetActorLocation`))
        (`KismetSystemLibrary.Delay` 2.0)
        (bind (_direction _mover) (`Timeline|Timeline`)
          (:`Update`
            (`self.K2_SetActorLocation` (`KismetMathLibrary.MakeVector` _locstart_x _locstart_y (`KismetMathLibrary.Lerp` _locstart_z 72.0 _mover)))))))))

(fn `UserConstructionScript`)