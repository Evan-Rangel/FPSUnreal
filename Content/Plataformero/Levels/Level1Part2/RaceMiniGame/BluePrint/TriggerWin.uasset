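; TriggerWin is the finish trigger of the race minigame in Level 1 Part 2 of the platformer.
; When BP_MasterChief overlaps it with at least three WinStars, it plays the MiniGameRace sound and fades the camera and audio out.
; After a delay timed near the end of the fade, it opens the PantallaWin level.
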(event `self.ReceiveBeginPlay`)

(event `self.ReceiveActorBeginOverlap`
  (params (OtherActor :type "Actor Object Reference"))
  (bind _asbp_master_chief (cast `/Game/Plataformero/Characters/MasterChief/BluePrints/BP_MasterChief` OtherActor))
  (if (>= (`/Game/Plataformero/Characters/MasterChief/BluePrints/BP_MasterChief.WinStars` _asbp_master_chief) 3)
    (`GameplayStatics.PlaySound2D` "/Game/Plataformero/Levels/Level1/SoundsANDMusic/MiniGameRace.MiniGameRace" 1.0 1.0 0.0 null null)
    (`PlayerCameraManager.StartCameraFade` :`self` (`GameplayStatics.GetPlayerCameraManager` 0) :`ToAlpha` 1.5 :`Duration` 6.2 :`bShouldFadeAudio` true)
    (`KismetSystemLibrary.Delay` 6.0)
    (`GameplayStatics.OpenLevel` "PantallaWin")))

(event `self.ReceiveActorEndOverlap`
  (params (OtherActor :type "Actor Object Reference"))
  (cast `/Game/Plataformero/Characters/MasterChief/BluePrints/BP_MasterChief` OtherActor))

(fn `UserConstructionScript`)