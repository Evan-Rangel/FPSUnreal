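; B_Door is a secret door Blueprint for a platformer level, driven by pressure switch events.
; SwitchActivate increments PressureSwitchNeeded and SwitchDeactivate decrements it, while PressureSwitchActive is only read.
; After each change, the OpenDoor timeline plays if Active is at least Needed and reverses otherwise.
; The timeline's DoorPosition track sets the relative Z of SecretDoor, sliding it vertically.
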(event `SwitchActivate`
  (`/Engine/EditorBlueprintResources/StandardMacros.IncrementInt` (`self.PressureSwitchNeeded`)
    (:`  `
      (if (>= (`self.PressureSwitchActive`) (`self.PressureSwitchNeeded`))
        (bind (_direction _doorposition) (`Timeline|OpenDoor` :!label _label)
          (:`Update`
            (`SceneComponent.K2_SetRelativeLocation` (`self.SecretDoor`) (`KismetMathLibrary.MakeVector` 0.0 0.0 _doorposition) false false)))
        (else
          (goto _label :!via `Reverse`))))))

(event `SwitchDeactivate`
  (`/Engine/EditorBlueprintResources/StandardMacros.DecrementInt` (`self.PressureSwitchNeeded`)
    (:`  `
      (if (>= (`self.PressureSwitchActive`) (`self.PressureSwitchNeeded`))
        (goto _label)
        (else
          (goto _label :!via `Reverse`))))))

(fn `UserConstructionScript`)