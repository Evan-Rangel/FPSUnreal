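; Player character for a platformer that collects win stars, spends Stars on buff and collector pickups, and gains a dash.
; Overlap casts route pickups, lap counters and the win trigger.
; Tick drives a timed coin minigame and an eight-lap race, which spawn collectors on success and reset on timeout.
; E talks to overlapping NPCs through dialogue interfaces and unconditionally starts the race, while Dash uses LaunchCharacter with temporarily altered ground friction.
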(event `self.ReceiveActorBeginOverlap`
  (params (OtherActor :type "Actor Object Reference"))
  (bind _stars (`self.Stars`))
  (bind _ascollector_to_win (cast `/Game/Plataformero/Levels/Level1/BluePrint/CollectorToWin` OtherActor)
    (:`then`
      (set `self.HaveCollector` true)
      (`self.K2_DestroyActor` _ascollector_to_win)
      (bind _result (`/Engine/EditorBlueprintResources/StandardMacros.IncrementInt` (`self.WinStars`))
        (:`  `
          (bind _output_get (set `self.WinStars` _result))
          (`KismetSystemLibrary.PrintString` (`KismetStringLibrary.Conv_IntToString` _output_get)))))
    (:`CastFailed`
      (bind _asspeed_buff (cast `/Game/Plataformero/Levels/Level1/BluePrint/SpeedBuff` OtherActor)
        (:`then`
          (if (>= _stars 12)
            (set `self.CanDash` true)
            (`self.K2_DestroyActor` _asspeed_buff)
            (set `self.Stars` (- (`self.Stars`) 12))))
        (:`CastFailed`
          (bind _ashealth_buff (cast `/Game/Plataformero/Levels/Level1/BluePrint/HealthBuff` OtherActor)
            (:`then`
              (if (>= _stars 5)
                (set `self.Health` (+ (`self.Health`) 1))
                (`self.K2_DestroyActor` _ashealth_buff)
                (set `self.Stars` (- (`self.Stars`) 12))))
            (:`CastFailed`
              (cast `/Game/Plataformero/Monedas/Blueprints/StarCoin_BP` OtherActor
                (:`then`
                  (if (`self.FlagMiigame`)
                    (set `self.StarsMinigame` (+ (`self.StarsMinigame`) 1))))
                (:`CastFailed`
                  (bind _ascollector_to_win_1shop (cast `/Game/Plataformero/Levels/Level1/BluePrint/CollectorToWin1Shop` OtherActor)
                    (:`then`
                      (if (>= (`self.Stars`) 50)
                        (`self.K2_DestroyActor` _ascollector_to_win_1shop)
                        (set `self.WinCollectors` (+ (`self.WinCollectors`) 1))
                        (set `self.Stars` (- (`self.Stars`) 50))
                        (set `self.HaveCollector` true)
                        (bind _result_2 (`/Engine/EditorBlueprintResources/StandardMacros.IncrementInt` (`self.WinStars`))
                          (:`  `
                            (bind _output_get_2 (set `self.WinStars` _result_2))
                            (`KismetSystemLibrary.PrintString` (`KismetStringLibrary.Conv_IntToString` _output_get_2))))))
                    (:`CastFailed`
                      (bind _asbp_lap_counter (cast `/Game/Plataformero/Levels/Level1Part2/RaceMiniGame/BluePrint/BP_LapCounter` OtherActor)
                        (:`then`
                          (if (`self.StartRaceMiniGame`)
                            (if (`/Game/Plataformero/Levels/Level1Part2/RaceMiniGame/BluePrint/BP_LapCounter.Activate` _asbp_lap_counter)
                              (set `self.Lap` (+ (`self.Lap`) 1))
                              (set `/Game/Plataformero/Levels/Level1Part2/RaceMiniGame/BluePrint/BP_LapCounter.Activate` false _asbp_lap_counter)
                              (`KismetArrayLibrary.Array_Add` (`self.ListLapCounter`) _asbp_lap_counter)
                              (if (== (`self.Lap`) 8)
                                (`self.SetActorHiddenInGame` false)
                                (`|SpawnActorFromClass` "/Game/Plataformero/Levels/Level1Part2/RaceMiniGame/BluePrint/Collector.Collector_C" (`KismetMathLibrary.Conv_VectorToTransform` (195.721842 -2406.107502 131.171826)) "Undefined" "OverrideRootScale" null null)
                                (set `self.StartRaceMiniGame` false)))))
                        (:`CastFailed`
                          (bind _ascollector (cast `/Game/Plataformero/Levels/Level1Part2/RaceMiniGame/BluePrint/Collector` OtherActor)
                            (:`then`
                              (bind _result_3 (`/Engine/EditorBlueprintResources/StandardMacros.IncrementInt` (`self.WinStars`))
                                (:`  `
                                  (set `self.WinStars` _result_3)
                                  (`self.K2_DestroyActor` _ascollector))))
                            (:`CastFailed`
                              (cast `/Game/Plataformero/Levels/Level1Part2/RaceMiniGame/BluePrint/TriggerWin` OtherActor)
                              (set `self.WinTrigger` (< (`self.WinStars`) 3)))))))))))))))))

(event `self.ReceiveBeginPlay`
  (`parent.ReceiveBeginPlay`)
  (set `self.Stars` 0)
  (bind _returnvalue (`|CreateWidget` "/Game/Plataformero/Characters/MasterChief/Ui/HUD_BP.HUD_BP_C"))
  (bind _output_get (set `self.UI` _returnvalue))
  (`UserWidget.AddToViewport` _output_get 0)
  (`self.SetMaxTime`)
  (set `self.TimerRace` (`self.MaxTimeRace`)))

(event `self.ReceiveTick`
  (params (DeltaSeconds :type "Float (single-precision)"))
  (`self.RaceTimer` DeltaSeconds)
  (if (`self.StartRaceMiniGame`)
    (bind _returnvalue (`|CreateWidget` "/Game/Plataformero/Levels/Level1Part2/RaceMiniGame/BluePrint/BPW_LapCounter.BPW_LapCounter_C" (`GameplayStatics.GetPlayerController` 0)))
    (bind _output_get (set `self.UIRace` _returnvalue))
    (`UserWidget.AddToViewport` _output_get 0)
    (set `self.ExistWRace` true)
    (elif (`self.ExistWRace`)
      (`Widget.RemoveFromParent` (`self.UIRace`))))
  (if (`self.ShowTimer`)
    (`self.TimerFunc` DeltaSeconds)
    (if (>= (`self.StarsMinigame`) (`self.StarsForNextLvl`))
      (set `self.NextRoom` true)
      (set `self.ShowTimer` false)
      (set `self.MinigameTrigger` false)
      (`|SpawnActorFromClass` "/Game/Plataformero/Levels/Level1/BluePrint/CollectorToWin.CollectorToWin_C" (`self.SpawnStar01`) "Undefined" "OverrideRootScale" null null)
      (elif (<= (`self.Time`) 0.0)
        (set `self.DestroyStars` true)
        (`self.SetMaxTime`)
        (set `self.Stars` (- (`self.Stars`) (`self.StarsMinigame`)))
        (set `self.StarsMinigame` 0)))))

(event `self.ReceiveActorEndOverlap`
  (params (OtherActor :type "Actor Object Reference"))
  (cast `/Game/Plataformero/Levels/Level1Part2/RaceMiniGame/BluePrint/TriggerWin` OtherActor)
  (set `self.WinTrigger` false))

(event `InputAction|Dash`
  (params (Key :type "Key Structure"))
  ;[1 1 1] Dash
  (:`Pressed`
    (if (`self.CanDash`)
      (`ActorComponent.SetActive` (`self.DashEffects`) true true)
      (`GameplayStatics.PlaySound2D` "/Game/Plataformero/Characters/MasterChief/Sounds/Dash.Dash" 1.0 1.0 0.0 null null)
      (`self.LaunchCharacter` (* (`self.GetLastMovementInputVector`) 300.0) true)
      (`self.SetMaxTime`))))

(event `self.OnLaunched`
  (params (LaunchVelocity :type "Vector Structure") (bXYOverride :type Boolean) (bZOverride :type Boolean))
  ;[1 1 1] Dash
  (set `CharacterMovementComponent.GroundFriction` -1.0 (`self.CharacterMovement`))
  (`KismetSystemLibrary.Delay` 0.3)
  (set `CharacterMovementComponent.GroundFriction` 8.0 (`self.CharacterMovement`))
  (`ActorComponent.SetActive` (`self.DashEffects`) false false)
  (`KismetSystemLibrary.Delay` 0.5))

(event `Key|E`
  (params (Key :type "Key Structure"))
  ;[1 1 1] Dialogo Sistem
  (:`Pressed`
    (`GameplayStatics.PlaySound2D` "/Game/Plataformero/Enemies/Fantasma2/Sounds/WomanGhostTalk.WomanGhostTalk" 1.0 1.0 0.0 null null)
    (for _array_element (`self.GetOverlappingActors` "/Game/Plataformero/DialogoSistem/BP_NPC.BP_NPC_C")
      (if (`KismetSystemLibrary.DoesImplementInterface` _array_element "/Game/Plataformero/DialogoSistem/BP_DialogoSistem.BP_DialogoSistem_C")
        (message `/Game/Plataformero/DialogoSistem/BP_DialogoSistem.Talk` _array_element)))
    (for _array_element_2 (`self.GetOverlappingActors` "/Game/Plataformero/DialogoSistem/BP_NPC2.BP_NPC2_C")
      (if (`KismetSystemLibrary.DoesImplementInterface` _array_element_2 "/Game/Plataformero/DialogoSistem/BP_DialogoSistem2.BP_DialogoSistem2_C")
        (message `/Game/Plataformero/DialogoSistem/BP_DialogoSistem2.Talk2` _array_element_2)))
    (set `self.StartRaceMiniGame` true)
    (for _array_element_3 (`self.GetOverlappingActors` "/Game/Plataformero/DialogoSistem/BP_NPC3.BP_NPC3_C")
      (if (`KismetSystemLibrary.DoesImplementInterface` _array_element_3 "/Game/Plataformero/DialogoSistem/BP_DialogoSistem3.BP_DialogoSistem3_C")
        (message `/Game/Plataformero/DialogoSistem/BP_DialogoSistem3.Talk3` _array_element_3)))))

(event `self.DamageTrigger.OnComponentBeginOverlap`
  (params (OverlappedComponent :type "PrimitiveComponent Object Reference") (OtherActor :type "Actor Object Reference") (OtherComp :type "PrimitiveComponent Object Reference") (OtherBodyIndex :type Integer) (bFromSweep :type Boolean) (SweepResult :type "HitResult Structure (by ref)"))
  (if (`self.CanDash`)
    (`GameplayStatics.ApplyDamage` OtherActor 1.0)
    (else
      (`GameplayStatics.ApplyDamage` null))))

(fn `AddStars`
  (params (NumberStars :type Integer))
  (set `self.Stars` (+ (`self.Stars`) NumberStars)))

(fn `RaceTimer`
  (params (NewParam :type "Float (double-precision)"))
  (bind _timerrace (`self.TimerRace`))
  (bind _listlapcounter (`self.ListLapCounter`))
  (if (`self.StartRaceMiniGame`)
    (set `self.TimerRace` (- _timerrace NewParam))
    (if (< _timerrace 0.0)
      (if (> (`KismetArrayLibrary.Array_Length` _listlapcounter) 0)
        (for _array_element _listlapcounter
          (set `/Game/Plataformero/Levels/Level1Part2/RaceMiniGame/BluePrint/BP_LapCounter.Activate` true _array_element)
          (set `self.Lap` 0 :!label _label)
          (set `self.TimerRace` (`self.MaxTimeRace`))
          (set `self.StartRaceMiniGame` false))
        (`KismetArrayLibrary.Array_Clear` _listlapcounter)
        (else
          (goto _label))))))

(fn `SetMaxTime`
  (set `self.Time` (`self.MaxTime`)))

(fn `TimerFunc`
  (params (DTime :type "Float (double-precision)"))
  (set `self.Time` (- (`self.Time`) DTime)))

(fn `UserConstructionScript`
  (`parent.UserConstructionScript`))